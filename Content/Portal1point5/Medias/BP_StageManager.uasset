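; Stage manager that handles streamed level transitions in a Portal-style game, loading the gel map from an empty level on BeginPlay.
; It spawns the portal manager and creates a loading widget at startup.
; LoadLevel disables player input, shows the loading animation and calls a dispatcher bound to LoadLevelEvent.
; That event unloads the current level, waits, resets portals and player position, streams in the next, then restores input and removes the widget.
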(event Custom|LoadLevelEvent
  (params (CurrentLevel :type Name) (NextLevel :type Name))
  (Game|UnloadStreamLevel(byName) CurrentLevel false)
  (Utilities|FlowControl|Delay 3.0)
  (Class|PortalManager|SetPortalsLocation (Variables|Default|GetPortalManager) "0, 0, 0")
  (Transformation|SetActorLocation (Game|Player|GetPlayerPawn 0) "0.000000,0.000000,-300.000000" false true)
  (Game|LoadStreamLevel(byName) NextLevel true)
  (Input|EnableInput (Game|Player|GetPlayerPawn 0) (Game|GetPlayerController 0))
  (Default|StopLoadingAnimation (Variables|Default|GetWidget_StageManager))
  (Widget|RemovefromParent (Variables|Default|GetWidget_StageManager)))

(event EventBeginPlay
  (EventDispatchers|BindEventtoLoadLevelDispatcher (delegate Custom|LoadLevelEvent))
  (bind _returnvalue (Game|SpawnActorfromClass "/Game/Portal1point5/Blueprints/BP_PortalManager.BP_PortalManager_C" (Math|Transform|MakeTransform "0, 0, 0" "0, 0, 0" "1.000000,1.000000,1.000000") "Undefined" "MultiplyWithRoot" 0 0))
  (Variables|Default|SetPortalManager _returnvalue)
  (bind _returnvalue_2 (UserInterface|CreateWidget "/Game/Portal1point5/Medias/WBP_StageManager.WBP_StageManager_C"))
  (Variables|Default|SetWidget_StageManager _returnvalue_2)
  (CallFunction|LoadLevel "L_Empty" "GameMap_Index5_UsingGel"))

(fn ConstructionScript)

(fn LoadLevel
  (params (CurrentLevel :type Name) (NextLevel :type Name))
  (Input|DisableInput (Game|Player|GetPlayerPawn 0) (Game|GetPlayerController 0))
  (UserInterface|Viewport|AddtoViewport (Variables|Default|GetWidget_StageManager) 1)
  (Default|StartLoadingAnimation (Variables|Default|GetWidget_StageManager))
  (Default|CallLoadLevelDispatcher CurrentLevel NextLevel))