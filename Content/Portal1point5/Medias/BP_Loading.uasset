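; Level-loading manager that streams in TitleMap on BeginPlay and swaps streamed levels behind a WBP_Loading fade overlay.
; LoadLevel rejects overlapping requests via a Loading flag, never cleared here, then fires a dispatcher that fades to dark and starts a delay timer.
; After the delay it unloads the old level, blocking-loads the new one, and polls on a looping timer, pausing until loaded, then fades in with game-only input.
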(event Custom|CustomEvent_1
  (params (OldLevel :type String) (NewLevel :type String))
  (Variables|Default|SetOldLevel OldLevel)
  (Variables|Default|SetNewLevel NewLevel)
  (Default|SetFade (Variables|Default|GetWBP_Loading) true 2.0)
  (Utilities|Time|SetTimerbyFunctionName 0 "DelayLoadLevel" 2.0))

(event Custom|CustomEvent_2
  (params (OldLevel :type String) (NewLevel :type String))
  (Game|UnloadStreamLevel(byName) (Utilities|String|StringToName OldLevel) false)
  (Game|LoadStreamLevel(byName) (Utilities|String|StringToName NewLevel) true true)
  (bind _returnvalue (Utilities|Time|SetTimerbyFunctionName 0 "WaitLoadLevel" 3.3e-05 true))
  (Variables|Default|SetTimerHandleLoadingLevel _returnvalue))

(event EventBeginPlay
  (Class|GameplayStatics|LoadStreamLevelbySoftObjectPtr "/Game/Portal1point5/Maps/TitleMap.TitleMap" true false)
  (bind _returnvalue (UserInterface|CreateWidget "/Game/Portal1point5/Medias/WBP_Loading.WBP_Loading_C"))
  (UserInterface|Viewport|AddtoViewport _returnvalue 1000)
  (Variables|Default|SetWBP_Loading _returnvalue)
  (EventDispatchers|BindEventtoLoadLevelProcess (delegate Custom|CustomEvent_1))
  (EventDispatchers|BindEventtoDelayLoadLevelProcess (delegate Custom|CustomEvent_2)))

(fn ConstructionScript)

(fn LoadLevel
  (params (OldLevel :type String) (NewLevel :type String))
  (if (Variables|Default|GetbLoading)
    (Development|PrintString "LoadError")
    (else
      (Variables|Default|SetbLoading true)
      (Default|CallLoadLevelProcess OldLevel NewLevel))))

(fn DelayLoadLevel
  (Default|CallDelayLoadLevelProcess (Variables|Default|GetOldLevel) (Variables|Default|GetNewLevel)))

(fn WaitLoadLevel
  (bind _returnvalue (Game|GetPlayerController 0))
  (if (Class|LevelStreaming|IsLevelLoaded (Class|GameplayStatics|GetStreamingLevel (Utilities|String|StringToName (Variables|Default|GetNewLevel))))
    (Game|SetGamePaused false)
    (Default|SetFade (Variables|Default|GetWBP_Loading) false 2.0)
    (Utilities|Time|ClearandInvalidateTimerbyHandle (Variables|Default|GetTimerHandleLoadingLevel))
    (Variables|/Script/Engine.PlayerController|SetbShowMouseCursor _returnvalue false)
    (Input|SetInputModeGameOnly _returnvalue false)
    (else
      (Game|SetGamePaused true))))