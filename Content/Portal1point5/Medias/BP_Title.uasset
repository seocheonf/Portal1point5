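; BP_Title sets up the title screen, showing its UI for as long as it is in play.
; On BeginPlay it creates a loading widget and stores it on BP_CustomGameInstance without displaying it.
; If that cast succeeds, it then creates the title widget, adds it to the viewport and switches the first player controller to UI-only input.
; EndPlay removes the title widget from its parent.
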(event EventBeginPlay
  (bind _returnvalue (UserInterface|CreateWidget "/Game/Portal1point5/Medias/WBP_Loading.WBP_Loading_C"))
  (bind _asbp_custom_game_instance (Utilities|Casting|CastToBP_CustomGameInstance (Game|GetGameInstance)))
  (Variables|/Game/Portal1point5/Medias/BP_CustomGameInstance.BP_CustomGameInstance_C|SetWBP_Loading _asbp_custom_game_instance _returnvalue)
  (bind _returnvalue_2 (UserInterface|CreateWidget "/Game/Portal1point5/Medias/WBP_Title.WBP_Title_C"))
  (bind _output_get (Variables|Default|SetWBP_Title _returnvalue_2))
  (UserInterface|Viewport|AddtoViewport _output_get 1)
  (Input|SetInputModeUIOnly (Game|GetPlayerController 0) 0 "DoNotLock" false))

(event EventEndPlay
  (params (EndPlayReason :type EEndPlayReason%20Enum :default "Destroyed"))
  (Widget|RemovefromParent (Variables|Default|GetWBP_Title)))

(fn ConstructionScript)