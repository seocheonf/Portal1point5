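; BP_StageEnd is the end-of-stage lift that closes behind the player and carries the stage out to the L_End level.
; When BP_PlayerCharacter overlaps the Sphere, a looping timer slides the Door shut.
; It then adds a WBP_Loading fade to dark and starts a second timer that raises the Platform, opening L_End at the top.
; Both motions use near-zero, once-per-frame timers scaled by delta seconds as a Tick substitute.
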(event OnComponentBeginOverlap(Sphere)
  (params (OverlappedComponent :type Primitive%20Component%20Object%20Reference) (OtherActor :type Actor%20Object%20Reference) (OtherComp :type Primitive%20Component%20Object%20Reference) (OtherBodyIndex :type Integer) (bFromSweep :type Boolean) (SweepResult :type Hit%20Result%20Structure%20%28by%20ref%29))
  (Utilities|Casting|CastToBP_PlayerCharacter OtherActor)
  (bind _returnvalue (Utilities|Time|SetTimerbyFunctionName 0 "DoorClosed" 3.3e-05 true true))
  (Variables|Default|SetHandle _returnvalue))

(fn ConstructionScript)

(fn DoorClosed
  (bind _door (Variables|Default|GetDoor))
  (Transformation|SetRelativeLocation _door (- (Variables|/Script/Engine.SceneComponent|GetRelativeLocation _door) (* (Class|KismetMathLibrary|VectorForward) (Utilities|Time|GetWorldDeltaSeconds) 200)) false false)
  (if (<= (.x (Variables|/Script/Engine.SceneComponent|GetRelativeLocation _door)) 0.0)
    (Utilities|Time|ClearandInvalidateTimerbyHandle (Variables|Default|GetHandle))
    (bind _returnvalue (Utilities|Time|SetTimerbyFunctionName 0 "PlatformUp" 3.3e-05 true true))
    (Variables|Default|SetHandle _returnvalue)
    (bind _returnvalue_2 (UserInterface|CreateWidget "/Game/Portal1point5/Medias/WBP_Loading.WBP_Loading_C"))
    (UserInterface|Viewport|AddtoViewport _returnvalue_2 10)
    (Default|SetFade _returnvalue_2 true 4.0)
    (Variables|Default|SetWidget_Loading _returnvalue_2)))

(fn PlatformUp
  (bind _platform (Variables|Default|GetPlatform))
  (Transformation|SetRelativeLocation _platform (+ (Variables|/Script/Engine.SceneComponent|GetRelativeLocation _platform) (* (Math|Vector|VectorUp) (Utilities|Time|GetWorldDeltaSeconds) 200)) false false)
  (if (>= (.z (Variables|/Script/Engine.SceneComponent|GetRelativeLocation _platform)) 8e+02)
    (Utilities|Time|ClearandInvalidateTimerbyHandle (Variables|Default|GetHandle))
    (Game|OpenLevel(byName) "L_End")))